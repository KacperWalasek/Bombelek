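; Bubble spawner actor that spawns actors at random intervals during play.
; Tick spawns once the game time passes the next spawn time, then reschedules it between minimum and maximum delays.
; Spawns ignore collision and take their transform from RandomizeBubbleTransform, whose graph builds a random XY point within the Box extents and a random uniform scale, though that node appears unconnected.
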(event `self.ReceiveTick`
  (params (DeltaSeconds :type "Float (single-precision)"))
  (if (> (`KismetSystemLibrary.GetGameTimeInSeconds`) (`self.NextBubbleSpawnTime`))
    (`self.UpdateSpawnTimers`)
    (`|SpawnActorFromClass` "/Game/Bubble/BP_Bubble.BP_Bubble_C" (`self.RandomizeBubbleTransform`) "AlwaysSpawn" "MultiplyWithRoot" null null)))

(event `self.ReceiveBeginPlay`
  (`self.UpdateSpawnTimers`))

(fn `UpdateSpawnTimers`
  (bind _output_get (set `self.PrevBubbleTime` (`KismetSystemLibrary.GetGameTimeInSeconds`)))
  (set `self.NextBubbleSpawnTime` (+ _output_get (`KismetMathLibrary.Lerp` (`self.MinSpawnTimeDifference`) (`self.MaxSpawnTimeDifference`) (`KismetMathLibrary.RandomFloat`)))))

(fn `UserConstructionScript`)