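; Spawner actor that releases BP_Bubble actors around its capsule at random intervals, moving horizontally.
; Tick checks a game-time threshold that UpdateSpawnTimers re-rolls between min and max delays on BeginPlay and after each spawn.
; RandomizeBubbleTransform1 uses random-angle trigonometry scaled by capsule radius for position, plus random uniform size and a separately randomized XY direction.
; Each new bubble receives that direction, then recalculates its force.
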(event `self.ReceiveTick`
  (params (DeltaSeconds :type "Float (single-precision)"))
  (if (> (`KismetSystemLibrary.GetGameTimeInSeconds`) (`self.NextBubbleSpawnTime`))
    (`self.UpdateSpawnTimers`)
    (bind (_transform _direction) (`self.RandomizeBubbleTransform1`))
    (bind _returnvalue (`|SpawnActorFromClass` "/Game/Bubble/BP_Bubble.BP_Bubble_C" _transform "AlwaysSpawn" "MultiplyWithRoot" null null))
    (set `/Game/Bubble/BP_Bubble.Direction` _direction _returnvalue)
    (`/Game/Bubble/BP_Bubble.RecalculateForce` _returnvalue)))

(event `self.ReceiveBeginPlay`
  (`self.UpdateSpawnTimers`))

(fn `RandomizeBubbleTransform1`
  (returns (Transform :type "Transform Structure") (Direction :type "Vector Structure"))
  (bind _returnvalue (`KismetMathLibrary.RandomFloatInRange` 0.0 360.0))
  (bind _returnvalue_2 (`KismetMathLibrary.MakeVector2D` (`KismetMathLibrary.DegCos` _returnvalue) (`KismetMathLibrary.DegSin` _returnvalue)))
  (return (`KismetMathLibrary.MakeTransform` (+ (`KismetMathLibrary.Conv_Vector2DToVector` (* _returnvalue_2 (`CapsuleComponent.GetScaledCapsuleRadius` (`self.Capsule`)))) (`SceneComponent.K2_GetComponentLocation` (`self.Capsule`))) (struct) (`KismetMathLibrary.Conv_DoubleToVector` (`KismetMathLibrary.RandomFloatInRange` (`self.MinBubbleSize`) (`self.MaxBubbleSize`)))) (`KismetMathLibrary.Conv_Vector2DToVector` _returnvalue_2)))

(fn `UpdateSpawnTimers`
  (bind _output_get (set `self.PrevBubbleTime` (`KismetSystemLibrary.GetGameTimeInSeconds`)))
  (set `self.NextBubbleSpawnTime` (+ _output_get (`KismetMathLibrary.Lerp` (`self.MinSpawnTimeDifference`) (`self.MaxSpawnTimeDifference`) (`KismetMathLibrary.RandomFloat`)))))

(fn `UserConstructionScript`)